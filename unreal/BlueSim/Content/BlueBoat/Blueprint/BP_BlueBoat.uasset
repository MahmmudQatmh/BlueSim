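; BP_BlueBoat is a physics-driven boat controllable by player input or ROS 2 velocity commands, with an onboard camera published to ROS 2.
; Each tick applies throttle as force and steering as yaw torque.
; Incoming Twist messages set both values and block triggered player input until commands stop for half a second.
; A looping timer captures the camera at about 30 Hz, with its render target handed to the ROS 2 publisher.
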(event `self.ReceiveEndPlay`
  (params (EndPlayReason :type "EEndPlayReason Enum" :default "Destroyed"))
  (`KismetSystemLibrary.PrintString` "ENDPLAY FIRED"))

(event `self.ReceiveBeginPlay`
  (bind _ros2node (`self.ROS2Node`))
  (bind _ros2node_2 (`self.ROS2Node`))
  (bind _ros2cmdvelsubscriber (`self.ROS2CmdVelSubscriber`))
  (bind _publisher (`ROS2PublisherComponent.Publisher` (`self.ROS2Publisher_Test`)))
  (`|ExecutionSequence`
    (:`then_0`
      (`EnhancedInputSubsystemInterface.AddMappingContext` (pcsubsystem `EnhancedInputLocalPlayerSubsystem` (`GameplayStatics.GetPlayerController` 0)) "/Game/BlueBoat/Input/IMC_Boat.IMC_Boat" 0 (struct))
      (`self.EnableInput` (`GameplayStatics.GetPlayerController` 0)))
    (:`then_1`
      (`KismetSystemLibrary.K2_SetTimerDelegate` (delegate `CaptureBoatCamera`) 0.0333 true))
    (:`then_2`
      (`ROS2NodeComponent.Init` _ros2node)
      (bind _asblue_sim_camera_publisher (cast `BlueSimCameraPublisher` _publisher))
      (set `BlueSimCameraPublisher.RenderTarget` "/Game/Sensors/RT_BoatCamera.RT_BoatCamera" _asblue_sim_camera_publisher)
      (set `BlueSimCameraPublisher.CaptureComponent` (`self.BoatCameraCapture`) _asblue_sim_camera_publisher)
      (set `BlueSimCameraPublisher.bFlipVertical` false _asblue_sim_camera_publisher)
      (`ROS2NodeComponent.AddPublisher` _ros2node _publisher))
    (:`then_3`
      (`ROS2NodeComponent.Init` _ros2node_2)
      (`ROS2NodeComponent.AddSubscription` _ros2node_2 (`ROS2SubscriberComponent.Subscriber` _ros2cmdvelsubscriber))
      (`ROS2Subscriber.SetDelegates` (`ROS2SubscriberComponent.Subscriber` _ros2cmdvelsubscriber) (delegate `OnCmdVelReceived`)))))

(event `EnhancedInput|/Game/BlueBoat/Input/IA_BoatThrottle`
  (params (ActionValue :type "Float (double-precision)") (ElapsedSeconds :type "Float (double-precision)") (TriggeredSeconds :type "Float (double-precision)") (InputAction :type "InputAction Object Reference" :default "/Game/BlueBoat/Input/IA_BoatThrottle.IA_BoatThrottle"))
  (:`Triggered`
    (bind _output_get (set `self.BoatThrottle` (select `bool` (`self.UseROSControl`) :`false` ActionValue :`true` (`self.BoatThrottle`)))))
  (:`Completed`
    (set `self.BoatThrottle` 0.0)))

(event `self.ReceiveTick`
  (params (DeltaSeconds :type "Float (single-precision)"))
  (bind _boatphysics (`self.BoatPhysics`))
  (`|ExecutionSequence`
    (:`then_0`
      (`PrimitiveComponent.AddForce` _boatphysics (`KismetMathLibrary.NegateVector` (* (`SceneComponent.GetRightVector` _boatphysics) (* (stale `EnhancedInput|/Game/BlueBoat/Input/IA_BoatThrottle` _output_get) 50000.0))) "None" false))
    (:`then_1`
      (`PrimitiveComponent.AddTorqueInDegrees` _boatphysics (`KismetMathLibrary.MakeVector` 0.0 0.0 (* (stale `EnhancedInput|/Game/BlueBoat/Input/IA_BoatSteering` _output_get) 30000000.0)) "None" false))
    (:`then_2`
      (if (> (- (`KismetSystemLibrary.GetGameTimeInSeconds`) (`self.LastROSCommandTime`)) 0.5)
        (set `self.UseROSControl` false)))))

(event `CaptureBoatCamera`
  (`SceneCaptureComponent2D.CaptureScene` (`self.BoatCameraCapture`)))

(event `EnhancedInput|/Game/BlueBoat/Input/IA_BoatSteering`
  (params (ActionValue :type "Float (double-precision)") (ElapsedSeconds :type "Float (double-precision)") (TriggeredSeconds :type "Float (double-precision)") (InputAction :type "InputAction Object Reference" :default "/Game/BlueBoat/Input/IA_BoatSteering.IA_BoatSteering"))
  (:`Triggered`
    (bind _output_get (set `self.BoatSteering` (select `bool` (`self.UseROSControl`) :`false` ActionValue :`true` (`self.BoatSteering`)))))
  (:`Completed`
    (set `self.BoatSteering` 0.0)))

(event `OnCmdVelReceived`
  (params (InMessage :type "ROS2GenericMsg Object Reference"))
  (bind _asros2twist_msg (cast `ROS2TwistMsg` InMessage))
  (`|ExecutionSequence`
    (:`then_0`
      (set `self.UseROSControl` true))
    (:`then_1`
      (bind (_linear _angular) (break `ROSTwist` (`ROS2TwistMsg.GetMsg` _asros2twist_msg)))
      (set `self.BoatThrottle` (.x _linear))
      (set `self.BoatSteering` (.z _angular)))))

(fn `UserConstructionScript`)