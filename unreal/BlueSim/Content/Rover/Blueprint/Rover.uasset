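; Player-driven rover Blueprint that moves a physics body through Enhanced Input, adding IMC_Rover on BeginPlay.
; Forward and backward apply force along the body's local Y axis, and releasing either zeroes linear velocity.
; Left and right yaw FrontAxis by the scaled input while turning the body at a fixed angular velocity, both reset on release.
; Tick zeroes both velocities whenever the body is below a hard-coded world height.
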(event `EnhancedInput|/Game/Rover/Input/IA_RoverForward`
  (params (ActionValue :type "Float (double-precision)") (ElapsedSeconds :type "Float (double-precision)") (TriggeredSeconds :type "Float (double-precision)") (InputAction :type "InputAction Object Reference" :default "/Game/Rover/Input/IA_RoverForward.IA_RoverForward"))
  (bind _roverphysics (`self.RoverPhysics`))
  (:`Triggered`
    (`PrimitiveComponent.AddForce` _roverphysics (* (`KismetMathLibrary.TransformDirection` (`SceneComponent.K2_GetComponentToWorld` _roverphysics) (`KismetMathLibrary.MakeVector` 0.0 -1.0)) (`self.RoverDriveForce`)) "None" false))
  (:`Completed`
    (`PrimitiveComponent.SetPhysicsLinearVelocity` (`self.RoverPhysics`) (0.0 0.0 0.0) false "None")))

(event `self.ReceiveBeginPlay`
  (`EnhancedInputSubsystemInterface.AddMappingContext` (pcsubsystem `EnhancedInputLocalPlayerSubsystem` (`GameplayStatics.GetPlayerController` 0)) "/Game/Rover/Input/IMC_Rover.IMC_Rover" 0 (struct)))

(event `EnhancedInput|/Game/Rover/Input/IA_RoverRight`
  (params (ActionValue :type "Float (double-precision)") (ElapsedSeconds :type "Float (double-precision)") (TriggeredSeconds :type "Float (double-precision)") (InputAction :type "InputAction Object Reference" :default "/Game/Rover/Input/IA_RoverRight.IA_RoverRight"))
  (bind _roverphysics (`self.RoverPhysics`))
  (:`Triggered`
    (`|ExecutionSequence`
      (:`then_0`
        (set `self.SteeringAngle` (* ActionValue (`self.MaxSteeringAngle`)))
        (`SceneComponent.K2_SetRelativeRotation` (`self.FrontAxis`) (`KismetMathLibrary.MakeRotator` 0.0 0.0 (`self.SteeringAngle`)) false false :!label _label))
      (:`then_1`
        (`PrimitiveComponent.SetPhysicsAngularVelocityInRadians` _roverphysics (0.0 0.0 0.8) false "None"))))
  (:`Completed`
    (`|ExecutionSequence`
      (:`then_0`
        (set `self.SteeringAngle` 0.0)
        (goto _label))
      (:`then_1`
        (`PrimitiveComponent.SetPhysicsAngularVelocityInRadians` _roverphysics (0.0 0.0 0.0) false "None")))))

(event `EnhancedInput|/Game/Rover/Input/IA_RoverLeft`
  (params (ActionValue :type "Float (double-precision)") (ElapsedSeconds :type "Float (double-precision)") (TriggeredSeconds :type "Float (double-precision)") (InputAction :type "InputAction Object Reference" :default "/Game/Rover/Input/IA_RoverLeft.IA_RoverLeft"))
  (bind _roverphysics (`self.RoverPhysics`))
  (:`Triggered`
    (`|ExecutionSequence`
      (:`then_0`
        (set `self.SteeringAngle` (* ActionValue (`self.MaxSteeringAngle`)))
        (goto _label))
      (:`then_1`
        (`PrimitiveComponent.SetPhysicsAngularVelocityInRadians` _roverphysics (0.0 0.0 -0.8) false "None"))))
  (:`Completed`
    (`|ExecutionSequence`
      (:`then_0`
        (set `self.SteeringAngle` 0.0)
        (goto _label))
      (:`then_1`
        (`PrimitiveComponent.SetPhysicsAngularVelocityInRadians` _roverphysics (0.0 0.0 0.0) false "None")))))

(event `self.ReceiveTick`
  (params (DeltaSeconds :type "Float (single-precision)"))
  (if (< (.z (`SceneComponent.K2_GetComponentLocation` (`self.RoverPhysics`))) 7400.0)
    (`PrimitiveComponent.SetPhysicsLinearVelocity` (`self.RoverPhysics`) (0.0 0.0 0.0) false "None")
    (`PrimitiveComponent.SetPhysicsAngularVelocityInRadians` (`self.RoverPhysics`) (0.0 0.0 0.0) false "None")))

(event `EnhancedInput|/Game/Rover/Input/IA_RoverBackward`
  (params (ActionValue :type "Float (double-precision)") (ElapsedSeconds :type "Float (double-precision)") (TriggeredSeconds :type "Float (double-precision)") (InputAction :type "InputAction Object Reference" :default "/Game/Rover/Input/IA_RoverBackward.IA_RoverBackward"))
  (bind _roverphysics (`self.RoverPhysics`))
  (:`Triggered`
    (`PrimitiveComponent.AddForce` _roverphysics (* (`KismetMathLibrary.TransformDirection` (`SceneComponent.K2_GetComponentToWorld` _roverphysics) (0.0 1.0 0.0)) (`self.RoverDriveForce`)) "None" false))
  (:`Completed`
    (`PrimitiveComponent.SetPhysicsLinearVelocity` (`self.RoverPhysics`) (0.0 0.0 0.0) false "None")))

(fn `UserConstructionScript`)